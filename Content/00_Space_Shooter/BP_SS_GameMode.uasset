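; Game mode for a space shooter that tracks kills, level and score progress, and starts the music on BeginPlay.
; Each destroyed enemy increments a counter, and every second kill raises Level by one.
; Puntuacion adds the given points to Progress, while PlayerDead casts the first player controller's HUD to BP_SpaceS_HUD and calls PlayerKilled on it.
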(event `PlayerDead`
  (bind _asbp_space_s_hud (cast `/Game/UI/BP_SpaceS_HUD` (`PlayerController.GetHUD` (`GameplayStatics.GetPlayerController` 0))))
  (`/Game/UI/BP_SpaceS_HUD.PlayerKilled` _asbp_space_s_hud))

(event `EnemyDestroyed`
  (bind _output_get (set `self.EnemiesDestroyed` (+ (`self.EnemiesDestroyed`) 1)))
  (if (== (mod _output_get 2) 0)
    (set `self.Level` (+ (`self.Level`) 1))))

(event `self.ReceiveBeginPlay`
  (`GameplayStatics.PlaySound2D` "/Game/Audio/musica.musica" 1.0 1.0 0.0 null null))

(event `self.ReceiveTick`
  (params (DeltaSeconds :type "Float (single-precision)")))

(event `Puntuacion`
  (params (Puntos :type Integer))
  (set `self.Progress` (+ (`self.Progress`) Puntos)))

(fn `UserConstructionScript`)