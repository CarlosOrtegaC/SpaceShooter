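; Base enemy for a space shooter that flies along its initial forward vector and fires Ammo from FirePoint on a timer.
; Tick drives movement and shooting.
; Overlapping the Player calls the OnEnemyDestroy dispatcher, updates game mode kills and score, damages the player and plays explosion effects.
; The bound handler destroys the enemy after a short delay, sometimes dropping BP_PowerVida; the ammo-cast path into the hit logic is unconnected.
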(event `self.ReceiveBeginPlay`
  (set `self.MovementVector` (`self.GetActorForwardVector`))
  (add `self.OnEnemyDestroy` (delegate `Destroyed_Event`)))

(event `Destroyed_Event`
  (`KismetSystemLibrary.Delay` 0.1)
  (if (>= (`KismetMathLibrary.RandomFloatInRange` 0.0 1.0) 0.6)
    (`|SpawnActorFromClass` "/Game/Enemies/BP_PowerVida.BP_PowerVida_C" (`SceneComponent.K2_GetComponentToWorld` (`self.FirePoint`)) "Undefined" "MultiplyWithRoot" null null))
  (`self.K2_DestroyActor`))

(event `self.ReceiveActorBeginOverlap`
  (params (OtherActor :type "Actor Object Reference"))
  (if (`KismetArrayLibrary.Array_Contains` (`Actor.Tags` OtherActor) "Player")
    (`self.OnEnemyDestroy`)
    (bind _asbp_ss_game_mode (cast `/Game/00_Space_Shooter/BP_SS_GameMode` (`GameplayStatics.GetGameMode`)))
    (`/Game/00_Space_Shooter/BP_SS_GameMode.EnemyDestroyed` _asbp_ss_game_mode)
    (`/Game/00_Space_Shooter/BP_SS_GameMode.Puntuacion` _asbp_ss_game_mode 1)
    (bind _asbp_sspace_s_character (cast `/Game/00_Space_Shooter/Players/BP_SSpaceS_Character` OtherActor))
    (`/Game/00_Space_Shooter/Players/BP_SSpaceS_Character.DamageActor` _asbp_sspace_s_character)
    (`GameplayStatics.SpawnEmitterAtLocation` "/Game/StarterContent/Particles/P_Explosion.P_Explosion" (`self.K2_GetActorLocation`))
    (`GameplayStatics.PlaySound2D` "/Game/StarterContent/Audio/Explosion02.Explosion02" 1.0 1.0 0.0 null null)))

(event `self.ReceiveTick`
  (params (DeltaSeconds :type "Float (single-precision)"))
  (`self.Move` DeltaSeconds)
  (bind _output_get (set `self.ShootCurrentTime` (+ DeltaSeconds (`self.ShootCurrentTime`))))
  (if (> _output_get (`self.DelayShoot`))
    (set `self.ShootCurrentTime` 0.0)
    (`self.Fire`)))

(fn `Fire`
  (bind _returnvalue (`|SpawnActorFromClass` (`self.Ammo`) (`SceneComponent.K2_GetComponentToWorld` (`self.FirePoint`)) "Undefined" "MultiplyWithRoot" null null))
  (`self.K2_SetActorRotation` _returnvalue (`self.K2_GetActorRotation`) false))

(fn `Move`
  (params (`Delta Time` :type "Float (double-precision)"))
  (`self.K2_SetActorLocation` (+ (`self.K2_GetActorLocation`) (* (* `Delta Time` (`self.Speed`)) (`self.MovementVector`)))))

(fn `UserConstructionScript`)