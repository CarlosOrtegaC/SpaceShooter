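; BP_PowerVida is a health power-up that drifts in a straight line and heals the player on contact.
; Tick calls Move, which offsets its location without sweep along the forward vector captured at BeginPlay, scaled by Speed.
; Overlapping a "Player" actor not tagged "Bala" fires OnPowerLife, then calls CurarPlayer on BP_SSpaceS_Character and plays particles and sound.
; Its own OnPowerLife binding destroys it after a short delay.
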(event `self.ReceiveBeginPlay`
  (set `self.MovementVector` (`self.GetActorForwardVector`))
  (add `self.onPowerLife` (delegate `Destroyed_Event`)))

(event `Destroyed_Event`
  (`KismetSystemLibrary.Delay` 0.1)
  (`self.K2_DestroyActor`))

(event `self.ReceiveActorBeginOverlap`
  (params (OtherActor :type "Actor Object Reference"))
  (bind _tags (`Actor.Tags` OtherActor))
  (if (`KismetArrayLibrary.Array_Contains` _tags "Player")
    (if (not (`KismetArrayLibrary.Array_Contains` _tags "Bala"))
      (`self.onPowerLife`)
      (bind _asbp_sspace_s_character (cast `/Game/00_Space_Shooter/Players/BP_SSpaceS_Character` OtherActor))
      (`/Game/00_Space_Shooter/Players/BP_SSpaceS_Character.CurarPlayer` _asbp_sspace_s_character)
      (`GameplayStatics.SpawnEmitterAtLocation` null (`self.K2_GetActorLocation`))
      (`GameplayStatics.PlaySound2D` null 1.0 1.0 0.0 null null))))

(event `self.ReceiveTick`
  (params (DeltaSeconds :type "Float (single-precision)"))
  (`self.Move` DeltaSeconds))

(fn `Move`
  (params (`Delta Time` :type "Float (double-precision)"))
  (`self.K2_SetActorLocation` (+ (`self.K2_GetActorLocation`) (* (* `Delta Time` (`self.Speed`)) (`self.MovementVector`)))))

(fn `UserConstructionScript`)