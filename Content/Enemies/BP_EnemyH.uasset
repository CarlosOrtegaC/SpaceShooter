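; BP_EnemyH is an enemy variant that bounces sideways between actors tagged "Wall".
; It sets the movement vector to its right vector at start, then flips it on each wall overlap using the IsRight flag.
; Each flip from right to left also shortens DelayShoot, with no lower clamp.
; Fire and construction only call the parent, and the file itself never applies the movement vector.
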(event `self.ReceiveBeginPlay`
  ;[1 1 1] Inicializa movimiento usando el vector derecho y define "Is Right".
  (`parent.ReceiveBeginPlay`)
  (set `self.MovementVector` (`self.GetActorRightVector`))
  (set `self.IsRight` true))

(event `self.ReceiveActorBeginOverlap`
  (params (OtherActor :type "Actor Object Reference"))
  (bind _returnvalue (`self.GetActorRightVector`))
  ;[1 1 1] Detecta colisión, ajusta movimiento y activa el retraso de disparo.
  (`parent.ReceiveActorBeginOverlap` OtherActor)
  (if (`KismetArrayLibrary.Array_Contains` (`Actor.Tags` OtherActor) "Wall")
    (if (`self.IsRight`)
      (set `self.IsRight` false)
      (set `self.MovementVector` (* _returnvalue -1.0))
      (set `self.DelayShoot` (- (`self.DelayShoot`) 0.1))
      (else
        (set `self.IsRight` true)
        (set `self.MovementVector` _returnvalue)))))

(fn `Fire`
  (`parent.Fire`))

(fn `UserConstructionScript`
  (`parent.UserConstructionScript`))